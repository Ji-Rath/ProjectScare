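; BP_Page is an interactable page actor that shows readable content on screen.
; OnInteract gets the base canvas from the player HUD, pushes a Widget_Readable onto its full-screen stack, and updates it from the PageData instanced struct when valid.
; Its Interactable interface reports a single-use type and an empty name, while CanInteract always returns false.
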(event OnInteract(Interactable)
  (params (Interactable :type Actor%20Object%20Reference) (Interactor :type Actor%20Object%20Reference) (Component :type Scene%20Component%20Object%20Reference))
  (bind _widget (Class|IBaseCanvasHolder|GetBaseCanvas(Message) (HUD|GetHUD (Game|GetPlayerController 0))))
  (bind _returnvalue (Class|CommonActivatableWidgetContainerBase|AddWidget (Variables|/Game/UI/WBP_BaseCanvas.WBP_BaseCanvas_C|GetFullScreenStack _widget) "/Game/UI/Widget_Readable.Widget_Readable_C"))
  (bind _value (Utilities|InstancedStruct|GetInstancedStructValue (Variables|Default|GetPageData))
    (:Valid
      (Class|ReadableWidget|UpdateReadable _returnvalue _value))))

(event EventBeginPlay)

(event Collision|EventActorBeginOverlap
  (params (OtherActor :type Actor%20Object%20Reference)))

(event EventTick
  (params (DeltaSeconds :type Float%20%28single-precision%29)))

(fn ConstructionScript)

(fn CanInteract
  (params (Interactor :type Actor%20Object%20Reference) (Component :type Scene%20Component%20Object%20Reference))
  (return false))

(fn GetInteractType
  (return "SingleUse"))

(fn GetName
  (params (Component :type Scene%20Component%20Object%20Reference))
  (return ""))