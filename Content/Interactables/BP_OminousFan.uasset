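; BP_OminousFan is a fan interactable with an on/off state that starts or stops its audio.
; Toggle and SetToggle route through the Interactable component's Interact, whose OnInteract event flips IsOn and calls UpdateState, which also runs on BeginPlay.
; CanInteract always returns false and the name is empty, so switching is left to callers of those two events.
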(event OnInteract(Interactable)
  (params (Interactable :type Actor%20Object%20Reference) (Interactor :type Actor%20Object%20Reference) (Component :type Scene%20Component%20Object%20Reference))
  (Variables|Default|SetIs%20On (not (Variables|Default|GetIs%20On)))
  (CallFunction|UpdateState))

(event EventBeginPlay
  (|CallParentFunction)
  (CallFunction|UpdateState))

(event Collision|EventActorBeginOverlap
  (params (OtherActor :type Actor%20Object%20Reference)))

(event EventTick
  (params (DeltaSeconds :type Float%20%28single-precision%29)))

(event EventToggle
  (Class|InteractableComponent|Interact (Variables|Default|GetInteractable) self))

(event EventSetToggle
  (params (bIsOn :type Boolean))
  (if (!= bIsOn (Variables|Default|GetIs%20On))
    (Class|InteractableComponent|Interact (Variables|Default|GetInteractable) self)))

(fn ConstructionScript)

(fn UpdateState
  (bind _audio (Variables|Default|GetAudio))
  (if (Variables|Default|GetIs%20On)
    (Audio|Components|Audio|Play _audio 0.0)
    (else
      (Audio|Components|Audio|Stop _audio))))

(fn CanInteract
  (params (Interactor :type Actor%20Object%20Reference) (Component :type Scene%20Component%20Object%20Reference))
  (return false))

(fn GetInteractType
  (return "SingleUse"))

(fn GetName
  (params (Component :type Scene%20Component%20Object%20Reference))
  (return ""))