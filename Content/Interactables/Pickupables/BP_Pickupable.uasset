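; Base pickup actor that adds one unit of its Item to the interactor's inventory on interact.
; Its construction script synchronously loads the item's mesh and applies the item's scale.
; The InteractableComponent's OnInteract event adds the item, sends a heads-up message through the message subsystem, plays a pickup sound and destroys the actor.
; Interaction queries report single use and an empty name, while CanInteract returns false.
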(event OnInteract(InteractableComponent)
  (params (Interactable :type Actor%20Object%20Reference) (Interactor :type Actor%20Object%20Reference) (Component :type Scene%20Component%20Object%20Reference))
  (Class|InventoryComponent|AddtoInventory (Actor|GetComponentbyClass Interactor "/Script/InteractionSystem.InventoryComponent") (Utilities|Struct|MakeItemData (Variables|Default|GetItem) 1))
  (bind _returnvalue (Utilities|InstancedStruct|MakeInstancedStruct (Variables|Default|GetPickupMessage)))
  (Class|MessageSubsystem|SendMessage (Subsystems|GetMessageSubsystem) "(TagName=\"Message.HeadsUp\")" _returnvalue)
  (Audio|PlaySoundatLocation (Variables|Default|GetPickupSound) (Transformation|GetActorLocation) "0, 0, 0" 1.0 1.0 0.0 0 0 0 0)
  (Actor|DestroyActor))

(event EventBeginPlay)

(event Collision|EventActorBeginOverlap
  (params (OtherActor :type Actor%20Object%20Reference)))

(event EventTick
  (params (DeltaSeconds :type Float%20%28single-precision%29)))

(fn ConstructionScript
  (bind _itemmesh (Variables|Components|GetItemMesh))
  (bind _item (Variables|Default|GetItem)
    (:then
      (bind _returnvalue (Utilities|LoadAssetBlocking (Variables|/Script/InteractionSystem.ItemInformation|GetItemMesh _item)))
      (bind _asstatic_mesh (Utilities|Casting|CastToStaticMesh _returnvalue))
      (Components|StaticMesh|SetStaticMesh _itemmesh _asstatic_mesh)
      (Transformation|SetRelativeScale3D _itemmesh (.Scale (Math|Transform|BreakTransform (Variables|/Script/InteractionSystem.ItemInformation|GetItemOffset _item)))))
    (:else)))

(fn CanInteract
  (params (Interactor :type Actor%20Object%20Reference) (Component :type Scene%20Component%20Object%20Reference))
  (return false))

(fn GetInteractType
  (return "SingleUse"))

(fn GetName
  (params (Component :type Scene%20Component%20Object%20Reference))
  (return ""))