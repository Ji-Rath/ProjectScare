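; Interactable hinged door that toggles open and closed on interact, swinging its hinge with a timeline, playing sounds and calling a door-interact notification.
; When locked, it searches the interactor's inventory for the required key, then either consumes it, unlocks and re-interacts, or plays a locked sound.
; Both outcomes send heads-up messages through the message subsystem.
; An equipped-item unlock variant exists but never runs.
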(event OnInteract(Interactable)
  (params (Interactable :type Actor%20Object%20Reference) (Interactor :type Actor%20Object%20Reference) (Component :type Scene%20Component%20Object%20Reference))
  (if (Variables|Door|GetbLocked)
    (|TryUnlockDoorSimple Interactor Component)
    (else
      (bind _output_get (Variables|Door|SetbIsOn (not (Variables|Door|GetbIsOn))))
      (Audio|SpawnSoundAttached (select _output_get "/Game/Interactables/Door/DoorOpen_Cue.DoorOpen_Cue" "/Game/Interactables/Door/DoorClose_Cue.DoorClose_Cue") (Variables|Default|GetDoorMesh) "None" "0, 0, 0" "0, 0, 0" "KeepRelativeOffset" false 1.0 1.0 0.0 0 0)
      (Default|CallOnDoorInteract Interactor)
      (if _output_get
        (bind _newtrack_0 (Timeline|OpenDoor Play)
          (:Update
            (Transformation|SetRelativeRotation (Variables|Default|GetDoorHinge) (Math|Rotator|MakeRotator 0.0 0.0 (* _newtrack_0 9e+01)) false false)))
        (else
          (Timeline|OpenDoor Reverse))))))

(event EventToggle
  (Class|InteractableComponent|Interact (Variables|Default|GetInteractable)))

(event EventSetToggle
  (params (bIsOn :type Boolean))
  (if (!= bIsOn (Variables|Door|GetbIsOn))
    (Class|InteractableComponent|Interact (Variables|Default|GetInteractable))))

(fn ConstructionScript)

(fn CanUnlockDoor
  (params (Item :type Item%20Information%20Object%20Reference))
  (return (== Item (Variables|Door|GetKeyRequired))))

(fn GetName
  (params (Component :type Scene%20Component%20Object%20Reference))
  (return ""))

(fn GetInteractType
  (return "SingleUse"))

(fn CanInteract
  (params (Interactor :type Actor%20Object%20Reference) (Component :type Scene%20Component%20Object%20Reference))
  (return true))