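; Player pawn that maps Enhanced Input actions to interaction, physics grabbing, equipped item use and drop, and a pause menu.
; The Interactor component outlines hovered actors through custom depth, while PhysicsGrab and PlayerEquip share the use-item input.
; Any damage immediately unpossesses the pawn and shows the game-over widget, with no health check.
; SPUD save and dialogue participant functions return fixed values, and the quick save/load calls are unwired.
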(event OnUpdateHover(Interactor)
  (params (Component :type Primitive%20Component%20Object%20Reference%20%28by%20ref%29))
  (Utilities|IsValid Component
    (:Is%20Valid
      (Variables|Default|GetInteractable
        (:then
          (Rendering|SetRenderCustomDepth (Actor|GetComponentbyClass (Variables|Default|GetInteractable) "/Script/Engine.StaticMeshComponent") false))
        (:else
          _))
      (Variables|Default|SetInteractable (Components|GetOwner Component))
      (Rendering|SetRenderCustomDepth (Actor|GetComponentbyClass (Variables|Default|GetInteractable) "/Script/Engine.StaticMeshComponent") true))
    (:Is%20Not%20Valid
      (Utilities|IsValid (Variables|Default|GetInteractable)
        (:Is%20Valid
          (Rendering|SetRenderCustomDepth (Actor|GetComponentbyClass (Variables|Default|GetInteractable) "/Script/Engine.StaticMeshComponent") false)
          (Variables|Default|SetInteractable 0))))))

(event Input|EnhancedActionEvents|EnhancedInputActionIA_Interact
  (params (ActionValue :type Boolean) (ElapsedSeconds :type Float%20%28double-precision%29) (TriggeredSeconds :type Float%20%28double-precision%29) (InputAction :type Input%20Action%20Object%20Reference :default "/Game/Input/IA_Interact.IA_Interact"))
  (Class|InteractorComponent|Interact (Variables|Default|GetInteractor)))

(event Input|EnhancedActionEvents|EnhancedInputActionIA_UseItem
  (params (ActionValue :type Boolean) (ElapsedSeconds :type Float%20%28double-precision%29) (TriggeredSeconds :type Float%20%28double-precision%29) (InputAction :type Input%20Action%20Object%20Reference :default "/Game/Input/IA_UseItem.IA_UseItem"))
  (:Started
    (Class|PhysicsGrabComponent|PhysicsInteract (Variables|Default|GetPhysicsGrab)))
  (:Completed
    (Class|PhysicsGrabComponent|ReleaseComponent (Variables|Default|GetPhysicsGrab))))

(event Input|EnhancedActionEvents|EnhancedInputActionIA_PushItem
  (params (ActionValue :type Boolean) (ElapsedSeconds :type Float%20%28double-precision%29) (TriggeredSeconds :type Float%20%28double-precision%29) (InputAction :type Input%20Action%20Object%20Reference :default "/Game/Input/IA_PushItem.IA_PushItem"))
  (Class|PhysicsGrabComponent|PushGrabbedComponent (Variables|Default|GetPhysicsGrab)))

(event Input|EnhancedActionEvents|EnhancedInputActionIA_DropItem
  (params (ActionValue :type Boolean) (ElapsedSeconds :type Float%20%28double-precision%29) (TriggeredSeconds :type Float%20%28double-precision%29) (InputAction :type Input%20Action%20Object%20Reference :default "/Game/Input/IA_DropItem.IA_DropItem"))
  (Class|PlayerEquipComponent|DropEquippedItem (Variables|Default|GetPlayerEquip)))

(event Input|EnhancedActionEvents|EnhancedInputActionIA_Pause
  (params (ActionValue :type Boolean) (ElapsedSeconds :type Float%20%28double-precision%29) (TriggeredSeconds :type Float%20%28double-precision%29) (InputAction :type Input%20Action%20Object%20Reference :default "/Game/Input/IA_Pause.IA_Pause"))
  (bind _asplayer_controller (Utilities|Casting|CastToPlayerController (Pawn|GetController)))
  (bind _widget (Class|IBaseCanvasHolder|GetBaseCanvas(Message) (HUD|GetHUD _asplayer_controller)))
  (Class|CommonActivatableWidgetContainerBase|AddWidget (Variables|/Game/UI/WBP_BaseCanvas.WBP_BaseCanvas_C|GetFullScreenStack _widget) "/Game/UI/Menu/Widget_Pause.Widget_Pause_C"))

(event Input|EnhancedActionEvents|EnhancedInputActionIA_UseItem
  (params (ActionValue :type Boolean) (ElapsedSeconds :type Float%20%28double-precision%29) (TriggeredSeconds :type Float%20%28double-precision%29) (InputAction :type Input%20Action%20Object%20Reference :default "/Game/Input/IA_UseItem.IA_UseItem"))
  (Class|PlayerEquipComponent|UseItem (Variables|Default|GetPlayerEquip)))

(event EventBeginPlay
  (|CallParentFunction)
  (Input|AddMappingContext (PlayerController|LocalPlayerSubsystems|GetEnhancedInputLocalPlayerSubsystem (CallFunction|GetPlayerController)) "/Game/Input/IMC_Player.IMC_Player" 0 "(bIgnoreAllPressedKeysUntilRelease=True,bForceImmediately=False,bNotifyUserSettings=False)"))

(event Game|Damage|EventAnyDamage
  (params (Damage :type Float%20%28single-precision%29) (DamageType :type Damage%20Type%20Object%20Reference) (InstigatedBy :type Controller%20Object%20Reference) (DamageCauser :type Actor%20Object%20Reference))
  (Pawn|UnPossess (Pawn|GetController))
  (bind _returnvalue (UserInterface|CreateWidget "/Game/UI/WBP_GameOver.WBP_GameOver_C"))
  (UserInterface|Viewport|AddtoPlayerScreen _returnvalue))

(fn ConstructionScript
  (|CallParentFunction)
  (Variables|Default|SetInventoryComp (Variables|Default|GetBP_Inventory))
  (Variables|Default|SetEquipComp (Variables|Default|GetPlayerEquip)))

(fn ShouldSkipRestoreVelocity
  (return false))

(fn ShouldSkipRestoreTransform
  (return false))

(fn GetSpudRespawnMode
  (return "Default"))

(fn GetPlayerController
  (bind _asplayer_controller (Utilities|Casting|CastToPlayerController (Pawn|GetController)))
  (return _asplayer_controller))

(fn CheckCondition
  (params (Context :type Dlg%20Context%20Object%20Reference) (ConditionName :type Name :default "None"))
  (return false))

(fn GetBoolValue
  (params (ValueName :type Name :default "None"))
  (return false))

(fn GetFloatValue
  (params (ValueName :type Name :default "None"))
  (return 0.0))

(fn GetIntValue
  (params (ValueName :type Name :default "None"))
  (return 0))

(fn GetNameValue
  (params (ValueName :type Name :default "None"))
  (return "None"))

(fn GetParticipantDisplayName
  (params (ActiveSpeaker :type Name :default "None"))
  (return "Self"))

(fn GetParticipantGender
  (return "Masculine"))

(fn GetParticipantIcon
  (params (ActiveSpeaker :type Name :default "None") (ActiveSpeakerState :type Name :default "None"))
  (return 0))

(fn GetParticipantName
  (return "Self"))

(fn ModifyBoolValue
  (params (ValueName :type Name :default "None") (bNewValue :type Boolean))
  (return false))

(fn ModifyFloatValue
  (params (ValueName :type Name :default "None") (bDelta :type Boolean) (Value :type Float%20%28single-precision%29))
  (return false))

(fn ModifyIntValue
  (params (ValueName :type Name :default "None") (bDelta :type Boolean) (Value :type Integer))
  (return false))

(fn ModifyNameValue
  (params (ValueName :type Name :default "None") (NameValue :type Name :default "None"))
  (return false))

(fn OnDialogueEvent
  (params (Context :type Dlg%20Context%20Object%20Reference) (EventName :type Name :default "None"))
  (return false))