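; UE5RFX function library for retro low-resolution rendering and vertex-light registration.
; The resolution function either lowers screen percentage to a target height with unfiltered upscaling, or sets Material Parameter Collection switches for fake UV pixelation, vertex snapping and dithering.
; Register and unregister functions edit the vertex light manager's actor-keyed map, packing scaled location with radius and brightness-multiplied color with normal influence.
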(fn UE5RFXResolutionSettings
  (params (TargetScreenHeight%20%28width%20gets%20calculated%29 :type Float%20%28single-precision%29) (UseScreenPercentage%28RealLowResolution%29 :type Boolean) (UseFakeResolutionForScreenSize%28VertexSnappingAndDithering%29 :type Boolean) (UseFakeResolutionForScreenUV%28FakePixelation%29 :type Boolean))
  (bind _returnvalue (Class|KismetSystemLibrary|MakeLiteralInteger))
  (bind _returnvalue_2 (Game|GetPlayerController 0 _returnvalue))
  (Rendering|Material|SetScalarParameterValue 0 "/Game/UE5RFX/Materials/UE5RFX_MaterialParameterCollection.UE5RFX_MaterialParameterCollection" "TargetResolutionHeight" TargetScreenHeight%20%28width%20gets%20calculated%29 :!class /Script/Engine.KismetMaterialLibrary)
  (Rendering|Material|SetScalarParameterValue 0 "/Game/UE5RFX/Materials/UE5RFX_MaterialParameterCollection.UE5RFX_MaterialParameterCollection" "ResolutionSwitchSize" :!class /Script/Engine.KismetMaterialLibrary)
  (Rendering|Material|SetScalarParameterValue 0 "/Game/UE5RFX/Materials/UE5RFX_MaterialParameterCollection.UE5RFX_MaterialParameterCollection" "ResolutionSwitchUV" :!class /Script/Engine.KismetMaterialLibrary)
  (if UseScreenPercentage%28RealLowResolution%29
    (Development|ExecuteConsoleCommand 0 (Utilities|String|Append "r.ScreenPercentage " (Utilities|String|ToString(Float) (/ (Math|Conversions|ToFloat(Integer) (Math|Float|Floor (* (/ TargetScreenHeight%20%28width%20gets%20calculated%29 (Math|Conversions|ToFloat(Integer) (.SizeY (HUD|GetViewportSize _returnvalue_2)))) 1e+04))) 1e+02))) _returnvalue_2)
    (Development|ExecuteConsoleCommand 0 "r.Upscale.Quality 0" _returnvalue_2)
    (else
      (Development|ExecuteConsoleCommand 0 (Utilities|String|Append "r.ScreenPercentage " "100") _returnvalue_2)
      (if UseFakeResolutionForScreenUV%28FakePixelation%29
        (Rendering|Material|SetScalarParameterValue 0 "/Game/UE5RFX/Materials/UE5RFX_MaterialParameterCollection.UE5RFX_MaterialParameterCollection" "ResolutionSwitchUV" 1.0 :!class /Script/Engine.KismetMaterialLibrary)
        (Rendering|Material|SetScalarParameterValue 0 "/Game/UE5RFX/Materials/UE5RFX_MaterialParameterCollection.UE5RFX_MaterialParameterCollection" "ResolutionSwitchSize" 1.0 :!class /Script/Engine.KismetMaterialLibrary :!label _label)
        (elif UseFakeResolutionForScreenSize%28VertexSnappingAndDithering%29
          (goto _label))))))

(fn UE5RFXRegisterVertexLight
  (params (Location :type Vector) (Radius :type Float%20%28double-precision%29) (LightColor :type Linear%20Color%20Structure) (Brightness :type Float%20%28single-precision%29) (NormalInfluence :type Float%20%28single-precision%29) (ActorToRegister :type Actor%20Object%20Reference%20%28by%20ref%29) (UseActorLocation :type Boolean))
  (bind _returnvalue (* LightColor Brightness))
  (bind _returnvalue_2 (/ Location 100))
  (bind (_r _g _b) (Math|Color|BreakColor _returnvalue))
  (bind _returnvalue_3 (Actor|GetActorOfClass 0 "/Game/UE5RFX/VertexLights/UE5RFX_VertexLight_Manager.UE5RFX_VertexLight_Manager_C"))
  (Utilities|Map|Add (Variables|/Game/UE5RFX/VertexLights/UE5RFX_VertexLight_Manager.UE5RFX_VertexLight_Manager_C|GetVertexLightArray _returnvalue_3) ActorToRegister (Utilities|Struct|MakeUE5RFX_VertexLightStruct (Math|Vector4|MakeVector4 (.x _returnvalue_2) (.y _returnvalue_2) (.z _returnvalue_2) Radius) (Math|Color|MakeColor _r _g _b NormalInfluence) UseActorLocation)))

(fn UE5RFXUnregisterVertexLight
  (params (ActorToUnregister :type Actor%20Object%20Reference%20%28by%20ref%29))
  (bind _returnvalue (Actor|GetActorOfClass 0 "/Game/UE5RFX/VertexLights/UE5RFX_VertexLight_Manager.UE5RFX_VertexLight_Manager_C"))
  (Utilities|Map|Remove (Variables|/Game/UE5RFX/VertexLights/UE5RFX_VertexLight_Manager.UE5RFX_VertexLight_Manager_C|GetVertexLightArray _returnvalue) ActorToUnregister))