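; Player character for the UE5RFX retro effects toolset, with Enhanced Input movement, look, camera zoom, jump, sprint and projectile shooting.
; BeginPlay applies a low screen-percentage resolution after a short delay, and the Use input cycles through real, faked and full-resolution modes.
; The flashlight toggles a looping timer that line-traces forward and registers a vertex light at the hit or trace end.
; Sprint branches on authority; auto-aim traces are unwired.
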(event Custom|EventFlashlight
  (bind _returnvalue (Transformation|GetActorLocation))
  (bind _outhit (Collision|LineTraceForObjects _returnvalue (+ _returnvalue (* (Transformation|GetActorForwardVector) 400)) (Utilities|Array|MakeArray "ObjectTypeQuery1") false 0 "None"))
  ;[1 0.8332 0.2123] Toggle light in manager
  (CallFunction|UE5RFXRegisterVertexLight (select (.bBlockingHit (Collision|BreakHitResult _outhit)) (.Location (Collision|BreakHitResult _outhit)) (.TraceEnd (Collision|BreakHitResult _outhit))) 4.2e+02 "(R=1.000000,G=0.756773,B=0.313022,A=1.000000)" 15.0 0.0 self false))

(event Custom|SprintServer
  (params (Max%20Walk%20Speed :type Float%20%28single-precision%29))
  (CallFunction|SprintClient Max%20Walk%20Speed))

(event Custom|SprintClient
  (params (Max%20Walk%20Speed :type Float%20%28single-precision%29))
  (Variables|/Script/Engine.CharacterMovementComponent|SetMaxWalkSpeed (Variables|Character|GetCharacterMovement) Max%20Walk%20Speed))

(event Input|EnhancedActionEvents|EnhancedInputActionIA_Flashlight
  (params (ActionValue :type Boolean) (ElapsedSeconds :type Float%20%28double-precision%29) (TriggeredSeconds :type Float%20%28double-precision%29) (InputAction :type Input%20Action%20Object%20Reference :default "/Game/UE5RFX/Blueprints/Gameplay/Input/IA_Flashlight.IA_Flashlight"))
  (:Started
    (Utilities|FlowControl|FlipFlop
      (:A
        (Utilities|Time|SetTimerbyFunctionName 0 "EventFlashlight" 0.1 true))
      (:B
        (Utilities|Time|ClearTimerbyFunctionName 0 "EventFlashlight")
        ;[1 0.8332 0.2123] Toggle light in manager
        (CallFunction|UE5RFXUnregisterVertexLight self)))))

(event Input|EnhancedActionEvents|EnhancedInputActionIA_Shoot
  (params (ActionValue :type Boolean) (ElapsedSeconds :type Float%20%28double-precision%29) (TriggeredSeconds :type Float%20%28double-precision%29) (InputAction :type Input%20Action%20Object%20Reference :default "/Game/UE5RFX/Blueprints/Gameplay/Input/IA_Shoot.IA_Shoot"))
  (bind _returnvalue (Transformation|GetActorRotation))
  (bind _returnvalue_2 (Math|Random|RandomFloatinRange -1.0 1.0))
  (bind _mesh (Variables|Character|GetMesh))
  (bind _returnvalue_3 (Transformation|GetSocketLocation _mesh "Head"))
  (:Started
    (Game|SpawnActorfromClass "/Game/UE5RFX/Blueprints/Gameplay/Projectile/UE5RFX_Projectile.UE5RFX_Projectile_C" (Math|Transform|MakeTransform _returnvalue_3 (Math|Rotator|MakeRotator (.roll _returnvalue) (+ (.pitch _returnvalue) _returnvalue_2) (+ (.yaw _returnvalue) _returnvalue_2)) "1.000000,1.000000,1.000000") "Undefined" "MultiplyWithRoot" 0 0)
    (Audio|PlaySoundatLocation "/Game/UE5RFX/Blueprints/Gameplay/Sounds/Freesound/750234__universfield__blaster-shot.750234__universfield__blaster-shot" _returnvalue_3 "0, 0, 0" 1.0 1.0 0.0 0 0 0 0)))

(event Input|EnhancedActionEvents|EnhancedInputActionIA_Sprint
  (params (ActionValue :type Boolean) (ElapsedSeconds :type Float%20%28double-precision%29) (TriggeredSeconds :type Float%20%28double-precision%29) (InputAction :type Input%20Action%20Object%20Reference :default "/Game/UE5RFX/Blueprints/Gameplay/Input/IA_Sprint.IA_Sprint"))
  (:Triggered
    (Networking|SwitchHasAuthority
      (:Authority
        (CallFunction|SprintClient 8e+02))
      (:Remote
        (CallFunction|SprintServer 8e+02))))
  (:Completed
    (Networking|SwitchHasAuthority
      (:Authority
        (CallFunction|SprintClient 2e+02))
      (:Remote
        (CallFunction|SprintServer 2e+02)))))

(event Input|EnhancedActionEvents|EnhancedInputActionIA_Use
  (params (ActionValue :type Boolean) (ElapsedSeconds :type Float%20%28double-precision%29) (TriggeredSeconds :type Float%20%28double-precision%29) (InputAction :type Input%20Action%20Object%20Reference :default "/Game/UE5RFX/Blueprints/Gameplay/Input/IA_Use.IA_Use"))
  (bind _returnvalue (Math|Float|MakeLiteralFloat 225.0))
  ;[0 1 0.2573] Resolution Settings
  (:Started
    (Utilities|FlowControl|MultiGate false true 1
      (:Out%200
        (CallFunction|UE5RFXResolutionSettings _returnvalue true false false)
        (Development|PrintString "Resolution Settings: Screen percentage"))
      (:Out%201
        (CallFunction|UE5RFXResolutionSettings _returnvalue false true false)
        (Development|PrintString "Resolution Settings: Full Resolution but Dithering and Vertex Snapping "))
      (:Out%202
        (CallFunction|UE5RFXResolutionSettings (Math|Float|MakeLiteralFloat 3.2e+02) false true true)
        (Development|PrintString "Resolution Settings: Full Resolution but faked low Resolution"))
      (:Out%203
        (CallFunction|UE5RFXResolutionSettings 224.0 false false false)
        (Development|PrintString "Resolution Settings: Full Resolution no special effects")))))

(event Input|EnhancedActionEvents|EnhancedInputActionIA_Jump
  (params (ActionValue :type Boolean) (ElapsedSeconds :type Float%20%28double-precision%29) (TriggeredSeconds :type Float%20%28double-precision%29) (InputAction :type Input%20Action%20Object%20Reference :default "/Game/UE5RFX/Blueprints/Gameplay/Input/IA_Jump.IA_Jump"))
  (:Triggered
    (Character|Jump))
  (:Completed
    (Character|StopJumping)))

(event Input|EnhancedActionEvents|EnhancedInputActionIA_Walk
  (params (ActionValue :type Vector%202D%20Structure) (ElapsedSeconds :type Float%20%28double-precision%29) (TriggeredSeconds :type Float%20%28double-precision%29) (InputAction :type Input%20Action%20Object%20Reference :default "/Game/UE5RFX/Blueprints/Gameplay/Input/IA_Walk.IA_Walk"))
  (bind _returnvalue (Pawn|GetControlRotation :!class /Script/Engine.Pawn))
  (bind (_x _y) (Math|Vector2D|BreakVector2D ActionValue))
  (bind _yaw (Math|Rotator|BreakRotator _returnvalue))
  (bind _returnvalue_2 (Math|Rotator|MakeRotator 0.0 0.0 _yaw))
  (Pawn|Input|AddMovementInput (Math|Vector|GetForwardVector _returnvalue_2) _x false)
  (Pawn|Input|AddMovementInput (Math|Vector|GetRightVector _returnvalue_2) _y false))

(event Input|EnhancedActionEvents|EnhancedInputActionIA_Zoom
  (params (ActionValue :type Float%20%28double-precision%29) (ElapsedSeconds :type Float%20%28double-precision%29) (TriggeredSeconds :type Float%20%28double-precision%29) (InputAction :type Input%20Action%20Object%20Reference :default "/Game/UE5RFX/Blueprints/Gameplay/Input/IA_Zoom.IA_Zoom"))
  (bind _springarm_camera (Variables|Default|GetSpringArm_Camera))
  (Variables|/Script/Engine.SpringArmComponent|SetTargetArmLength _springarm_camera (Math|Float|Clamp(Float) (+ (Variables|/Script/Engine.SpringArmComponent|GetTargetArmLength _springarm_camera) (* ActionValue -1e+01)) 1e+02 1e+03)))

(event Input|EnhancedActionEvents|EnhancedInputActionIA_Look
  (params (ActionValue :type Vector%202D%20Structure) (ElapsedSeconds :type Float%20%28double-precision%29) (TriggeredSeconds :type Float%20%28double-precision%29) (InputAction :type Input%20Action%20Object%20Reference :default "/Game/UE5RFX/Blueprints/Gameplay/Input/IA_Look.IA_Look"))
  (bind (_x _y) (Math|Vector2D|BreakVector2D ActionValue))
  (Pawn|Input|AddControllerYawInput _x)
  (Pawn|Input|AddControllerPitchInput (* _y -1.0)))

(event EventBeginPlay
  ;[0.05613 0.1441 0.2307] BeginPlayEvent
  (bind _asplayer_controller (Utilities|Casting|CastToPlayerController (Pawn|GetController)))
  (Input|AddMappingContext (PlayerController|LocalPlayerSubsystems|GetEnhancedInputLocalPlayerSubsystem _asplayer_controller) "/Game/UE5RFX/Blueprints/Gameplay/Input/Input_MappingContext.Input_MappingContext" 0 "(bIgnoreAllPressedKeysUntilRelease=True,bForceImmediately=False,bNotifyUserSettings=False)")
  ;[0 1 0.2573] Resolution Settings
  ;;[1 1 1] Delay needed or it gets not triggered ingame
  (Utilities|FlowControl|Delay 0.5)
  (CallFunction|UE5RFXResolutionSettings (Math|Float|MakeLiteralFloat 225.0) true false false)
  (Development|PrintString "Resolution Settings: Screen percentage"))

(event EventOnLanded
  (params (Hit :type Hit%20Result%20Structure%20%28by%20ref%29))
  (Audio|PlaySoundatLocation "/Game/UE5RFX/Blueprints/Gameplay/Sounds/Freesound/477355__nuff3__steps-tile-falling_1a.477355__nuff3__steps-tile-falling_1a" (Transformation|GetActorLocation) "0, 0, 0" 1.0 1.0 0.0 0 0 0 0))

(event Input|KeyboardEvents|DebugKeyF12
  (params (Key :type Key%20Structure) (ActionValue :type Input%20Action%20Value%20Structure))
  (:Pressed
    (Development|ExecuteConsoleCommand "shot" 0)))

(fn ConstructionScript)