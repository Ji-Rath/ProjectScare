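; Child actor that gives its parent actor a projected shadow by rendering it to a texture on a decal mesh.
; A scene capture showing only the parent writes to a runtime-created render target with nearest filtering, which feeds the decal's dynamic material.
; Decal size drives both mesh scale and capture ortho width.
; Setup runs in construction and at BeginPlay; animated shadows recapture on a looping timer rather than every frame.
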(event Custom|Shadowinitialization
  (bind _shadowdecalsize (Variables|Default|GetShadowDecalSize))
  (bind _ue5rfx_shadowcapture (Variables|Default|GetUE5RFX_ShadowCapture))
  (bind _ue5rfx_decal_mesh (Variables|Default|GetUE5RFX_Decal_Mesh))
  (bind _shadowresolution (Variables|Default|GetShadowResolution))
  (Variables|/Script/Engine.SceneCaptureComponent|SetShowOnlyActors (Variables|Default|GetUE5RFX_ShadowCapture) (Utilities|Array|MakeArray (Actor|GetParentActor)))
  (Transformation|SetWorldScale3D (Variables|Default|GetUE5RFX_Decal_Mesh) (Math|Conversions|ToVector(Float) (/ _shadowdecalsize 100)))
  (bind _returnvalue (Rendering|CreateRenderTarget2D _shadowresolution _shadowresolution "RTF_RGBA8_SRGB"))
  (bind _output_get (Variables|Default|SetRenderTarget _returnvalue))
  (Variables|/Script/Engine.Texture|SetFilter _output_get "TF_Nearest")
  (Variables|/Script/Engine.SceneCaptureComponent2D|SetTextureTarget _ue5rfx_shadowcapture _output_get)
  (Variables|/Script/Engine.SceneCaptureComponent2D|SetOrthoWidth _ue5rfx_shadowcapture (Math|Conversions|ToFloat(Integer) _shadowdecalsize))
  (bind _returnvalue_2 (Rendering|Material|CreateDynamicMaterialInstance _ue5rfx_decal_mesh 0 (Rendering|Material|GetMaterial _ue5rfx_decal_mesh 0) "None" :!class /Script/Engine.PrimitiveComponent))
  (Variables|Default|SetShadowMaterial _returnvalue_2)
  (Rendering|Material|SetTextureParameterValue _returnvalue_2 "ShadowTexture" (Variables|Default|GetRenderTarget))
  (CallFunction|CaptureShadow))

(event Custom|CaptureShadow
  (Rendering|SceneCapture|CaptureScene (Variables|Default|GetUE5RFX_ShadowCapture) :!class /Script/Engine.SceneCaptureComponent2D))

(event EventBeginPlay
  (CallFunction|Shadowinitialization)
  (if (Variables|Default|GetIsAnimated)
    (Utilities|Time|SetTimerbyEvent (delegate Custom|CaptureShadow) 0.1 true)))

(fn ConstructionScript
  (CallFunction|Shadowinitialization))