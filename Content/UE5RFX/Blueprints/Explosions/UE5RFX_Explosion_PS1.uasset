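; UE5RFX PS1-style explosion actor that plays a one-shot effect, sound and radial damage with falloff on spawn, then destroys itself.
; A timeline at adjustable play rate scales a randomly rotated sphere mesh and feeds time to the sphere and sprite through Custom Primitive Data.
; The timeline also optionally registers a colored vertex light each update.
; Sphere overlaps only print the hit actor's name.
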(event OnComponentBeginOverlap(StaticMesh_ExplosionSphere)
  (params (OverlappedComponent :type Primitive%20Component%20Object%20Reference) (OtherActor :type Actor%20Object%20Reference) (OtherComp :type Primitive%20Component%20Object%20Reference) (OtherBodyIndex :type Integer) (bFromSweep :type Boolean) (SweepResult :type Hit%20Result%20Structure%20%28by%20ref%29))
  (Development|PrintString (Utilities|String|Append "Hit Actor: " (Utilities|GetDisplayName OtherActor))))

(event EventBeginPlay
  (bind _explosionsize (Variables|Default|GetExplosionSize))
  (Transformation|SetRelativeRotation (Variables|Default|GetStaticMesh_ExplosionSphere) (Math|Random|RandomRotator true) false false)
  (Components|Timeline|SetPlayRate (Variables|Default|GetTimeline) (Variables|Default|GetExplosionPlayRate))
  (Audio|PlaySoundatLocation "/Game/UE5RFX/Blueprints/Gameplay/Sounds/Freesound/514133__juverisetila__medium-explosion.514133__juverisetila__medium-explosion" (Transformation|GetActorLocation) "0, 0, 0" 1.0 1.0 0.0 0 0 0 0)
  ;[1 0.02 0 0.5] Damage Event
  (Class|GameplayStatics|ApplyRadialDamagewithFalloff (Variables|Default|GetBase%20Damage) (Variables|Default|GetMinimum%20Damage) (Transformation|GetActorLocation) (Variables|Default|GetDamage%20Inner%20Radius) (Variables|Default|GetDamage%20Outer%20Radius) (Variables|Default|GetDamage%20Falloff) (Variables|Default|GetDamage%20Type%20Class) (Variables|Default|GetIgnore%20Actors) (Variables|Default|GetDamage%20Causer) (Variables|Default|GetInstigated%20by%20Controller) (Variables|Default|GetDamage%20Prevention%20Channel))
  (Rendering|Material|SetCustomPrimitiveDataFloat (Variables|Default|GetStaticMesh_ExplosionSprite) 1 _explosionsize)
  (bind (_direction _time _lightcolor) (Timeline|Timeline Play)
    (:Update
      (Rendering|Material|SetCustomPrimitiveDataFloat (Variables|Default|GetStaticMesh_ExplosionSprite) 0 _time)
      (Transformation|SetWorldScale3D (Variables|Default|GetStaticMesh_ExplosionSphere) (Math|Conversions|ToVector(Float) (* _time _explosionsize)))
      (if (Variables|Default|GetDrawVertexLight)
        (CallFunction|UE5RFXRegisterVertexLight (Transformation|GetActorLocation) (Variables|Default|GetExplosionSize) _lightcolor 12.0 0.0 self false)))
    (:Finished
      (Actor|DestroyActor))))

(fn ConstructionScript)